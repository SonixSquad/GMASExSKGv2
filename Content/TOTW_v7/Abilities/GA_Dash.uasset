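; GA_Dash is a dash ability built on the GMC (General Movement Component) ability framework, currently an unfinished stub.
; On begin, it casts the owner's movement component to GMCE_OrganicMovementCmp and does nothing further.
; Disconnected nodes hold a launch-to-location call followed by cost and cooldown commit and ability end, plus a bound-bool check with no action.
; As wired, it never moves the character, commits cost or ends itself.
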(event `self.BeginAbilityEvent`
  (bind _asgmcextended_organic_movement_component (cast `GMCE_OrganicMovementCmp` (`GMC_AbilitySystemComponent.GMCMovementComponent` (`self.OwnerAbilityComponent`)))))