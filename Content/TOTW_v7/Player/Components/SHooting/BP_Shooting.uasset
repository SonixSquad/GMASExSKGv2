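; Player shooting component that runs semi/full-auto hitscan fire for SKG firearms, networked through General Movement Component (GMC) bound variables.
; ShootingTick gates shots by fire rate, then line-traces from the muzzle along control rotation.
; The server validates client-reported hit actors with lag-compensation rewind, sphere traces and blocker checks, then applies GMAS effects to Saboteur-tagged targets.
; ShootSimulated reproduces muzzle, beam and impact effects from the replicated hit actor.
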(event `self.ReceiveBeginPlay`
  (`parent.ReceiveBeginPlay`)
  (set `self.SKGWeaponHandlingRef` (`Actor.GetComponentByClass` (`self.GetOwner`) "/Script/SKGShooterFramework.SKGShooterPawnComponent"))
  (bind _asbp_skgpawn_char (cast `/Game/TOTW_v7/Characters/BP_SKGPawn_Char` (`self.GetOwner`)))
  (bind _output_get (set `self.OuterPawn` _asbp_skgpawn_char))
  (bind _asplayer_controller (cast `PlayerController` (`Pawn.GetController` _output_get)))
  (bind _returnvalue (pcsubsystem `EnhancedInputLocalPlayerSubsystem` _asplayer_controller))
  (`/Engine/EditorBlueprintResources/StandardMacros.IsValid` _returnvalue
    (:`Is Valid`
      (`EnhancedInputSubsystemInterface.AddMappingContext` _returnvalue "/Game/GMASExtended/Input/IC_Basic.IC_Basic" 0 (struct)))))

(event `BindReplicationData`
  (params (Outer :type "/Game/GMASExtended/Blueprints/BP_ExampleMovement Object Reference"))
  (bind _output_get (set `self.OuterComponent` Outer))
  (`GMC_ReplicationCmp.BindBool` _output_get (`self.WantsToShoot`) "ClientAuth_Input" "CombineIfUnchanged" "None" "NearestNeighbour")
  (`GMC_ReplicationCmp.BindBool` _output_get (`self.SimulateShot`) "Local" "AlwaysCombine" "Periodic_Output" "NearestNeighbour")
  (`GMC_ReplicationCmp.BindActorReference` _output_get (`self.HitActorSimulated`) "Local" "AlwaysCombine" "Periodic_Output" "NearestNeighbour")
  (bind _returnvalue (`GMC_ReplicationCmp.BindActorReference` _output_get (`self.RemoteHitActor`) "ClientAuth_Output" "AlwaysCombine" "None" "NearestNeighbour"))
  (set `self.BI_RemoteHitActor` _returnvalue))

(event `EnhancedInput|/Game/GMASExtended/Input/IA_Fire`
  (params (ActionValue :type Boolean) (ElapsedSeconds :type "Float (double-precision)") (TriggeredSeconds :type "Float (double-precision)") (InputAction :type "InputAction Object Reference" :default "/Game/GMASExtended/Input/IA_Fire.IA_Fire"))
  ;[0.009006 0.2124 0.8646] trigger
  (:`Triggered`
    (set `self.WantsToShoot` true))
  (:`Completed`
    (set `self.WantsToShoot` false)))

(event `EnhancedInput|/Game/GMASExtended/Input/IA_CycleFireMode`
  (params (ActionValue :type Boolean) (ElapsedSeconds :type "Float (double-precision)") (TriggeredSeconds :type "Float (double-precision)") (InputAction :type "InputAction Object Reference" :default "/Game/GMASExtended/Input/IA_CycleFireMode.IA_CycleFireMode"))
  ;[0.009006 0.2124 0.8646] Semi Auto / Full Auto toggle
  (:`Triggered`
    (`/Engine/EditorBlueprintResources/StandardMacros.FlipFlop`
      (:`A`
        (set `self.SemiAuto` false))
      (:`B`
        (set `self.SemiAuto` true)))))

(event `ShootingTick`
  (params (DeltaTime :type "Float (single-precision)") (LocalMove :type Boolean) (CombinedClientMove :type Boolean))
  ;[0.5365 0.437 0] Shooting Tick
  (`self.PreShoot`)
  (bind (_shouldshoot _fireratepause) (`self.ShouldShoot` (`self.WantsToShoot`) (`self.SemiAuto`) (`self.FireRate`) (`GMC_MovementUtilityCmp.GetMoveTimestamp` (`self.OuterComponent`))))
  (if _shouldshoot
    (bind (_hit _hitpawn _hitlocation _hitactor) (`self.Shoot`))
    ;[1 0 0.03767] Enemy Detection via tags
    (`/Engine/EditorBlueprintResources/StandardMacros.IsValid` _hitactor
      (:`Is Valid`
        (bind _returnvalue (`Actor.GetComponentByClass` _hitactor "/Script/GMCAbilitySystem.GMC_AbilitySystemComponent"))
        (`/Engine/EditorBlueprintResources/StandardMacros.IsValid` _returnvalue
          (:`Is Valid`
            (if (`GMC_AbilitySystemComponent.HasActiveTag` _returnvalue (struct :`TagName` "Identity.Faction.Saboteur"))
              ;[0.009006 0.2124 0.8646] Apply Damage GMAS method
              (bind _shouldapplydamage (`self.ShouldApplyDamage` _hitactor))
              (if _shouldapplydamage
                (`GMC_AbilitySystemComponent.ApplyAbilityEffectSafe` :`self` _returnvalue :`QueueType` "Predicted"))
              (else
                (`KismetSystemLibrary.PrintString` "NOT AN ENEMY!" true true (struct :`G` 0.296875 :`B` 0.010464 :`A` 1.0) 0.3)))))))
    (else
      (`self.DoNotShoot` _fireratepause DeltaTime))))

(fn `CheckCurrentFirearm`
  (returns (CurrentFirearmComponent :type "SKGFirearmComponent Object Reference"))
  (bind _returnvalue (`SKGShooterPawnComponent.GetCurrentFirearmComponent` (`SKGShooterPawnComponent.GetShooterPawnComponent` (`self.OuterPawn`))))
  (`/Engine/EditorBlueprintResources/StandardMacros.IsValid` _returnvalue
    (:`Is Valid`
      (return _returnvalue))))

(fn `CL_SetHitActor`
  (params (HitActor :type "Actor Object Reference") (HitPawn :type Boolean))
  (bind _cl_savedhitactor (`self.CL_SavedHitActor`))
  (if (`self.CL_ShouldCombineHits` HitActor)
    (if (`GMC_MovementUtilityCmp.IsCombinedMove` (`self.OuterComponent`))
      (if (`self.CL_ShouldEnqueueNewMove` (`local.HitPawn`) (`local.HitActor`) (`self.CL_SavedHitActor`))
        (`GMC_ReplicationCmp.CL_DoNotCombineNextMove` (`self.OuterComponent`)))
      (if (`KismetSystemLibrary.IsValid` _cl_savedhitactor)
        (set `self.RemoteHitActor` _cl_savedhitactor)
        (else
          (if (`local.HitPawn`) :!label _label
            (bind _output_get (set `self.RemoteHitActor` (`local.HitActor`)))
            (set `self.CL_SavedHitActor` _output_get)
            (else
              (set `self.RemoteHitActor` null)
              (set `self.CL_SavedHitActor` null)))))
      (else
        (goto _label)))
    (elif (`local.HitPawn`)
      (`GMC_ReplicationCmp.CL_DoNotCombineNextMove` (`self.OuterComponent`))
      (goto _label)
      (else
        (goto _label)))))

(fn `CL_ShouldCombineHits`
  (params (HitActor :type "Actor Object Reference"))
  (returns (ShouldCombineHits :type Boolean))
  ;[1 0.05 0] It is advisable to combine shots when the target receives a lot of consecutive hits with a high fire rate weapon. Hit detection is less accurate (more lenient) when shots are combined.
  (return false))

(fn `CL_ShouldEnqueueNewMove`
  (params (HitPawn :type Boolean) (HitActor :type "Actor Object Reference") (SavedHitActor :type "Actor Object Reference"))
  (returns (ShouldEnqueueNewMove :type Boolean))
  (if (and HitPawn (!= HitActor SavedHitActor))
    _
    (elif (and (not HitPawn) (`KismetSystemLibrary.IsValid` SavedHitActor))
      _
      (else
        (return false))))
  (return true))

(fn `DoNotShoot`
  (params (FireRatePause :type Boolean) (DeltaTime :type "Float (double-precision)"))
  (bind _returnvalue (< (`self.SV_ShotReplicationTimer`) 0.1))
  (`/Engine/EditorBlueprintResources/ActorComponentMacros.Switch Has Authority`
    (:`Authority`
      (bind _output_get (set `self.SV_ShotReplicationTimer` (+ (stale _output_get) (`local.DeltaTime`))))
      (if (`self.SemiAuto`)
        (set `self.SimulateShot` _returnvalue :!label _label)
        (elif (not (`self.WantsToShoot`))
          (goto _label)
          (else
            (set `self.SimulateShot` true))))
      (if (not _returnvalue)
        (set `self.HitActorSimulated` null)))
    (:`Remote`
      (if (`local.FireRatePause`)
        (set `self.RemoteHitActor` (stale _output_get_2))
        (else
          (bind _output_get_2 (set `self.CL_SavedHitActor` null)))))))

(fn `GetShootingTracePoints`
  (returns (TraceStart :type "Vector Structure") (TraceEnd :type "Vector Structure") (AimPoint :type "Transform Structure"))
  (bind _returnvalue_location (`KismetMathLibrary.BreakTransform` (`SKGFirearmComponent.GetMuzzleTransform` (`SKGShooterPawnComponent.GetCurrentFirearmComponent` (`SKGShooterPawnComponent.GetShooterPawnComponent` (`self.OuterPawn`))))))
  (return _returnvalue_location (+ _returnvalue_location (* (`KismetMathLibrary.Conv_RotatorToVector` (`GMC_ReplicationCmp.GetControlRotationWorldSpace` (`self.OuterComponent`))) (`self.Range`)))))

(fn `PlayShootFX`
  (params (Hit :type Boolean) (HitPawn :type Boolean) (HitLocation :type "Vector Structure") (Firearm :type "/Game/SKGSFExampleContent/Blueprints/Firearms/BP_Firearm Object Reference"))
  (bind _returnvalue (`KismetMathLibrary.RandomFloatInRange` 0.5 0.8))
  (bind (_returnvalue_location _returnvalue_rotation) (`KismetMathLibrary.BreakTransform` (`SKGFirearmComponent.GetMuzzleTransform` (`SKGShooterPawnComponent.GetCurrentFirearmComponent` (`SKGShooterPawnComponent.GetShooterPawnComponent` (`self.OuterPawn`))))))
  (set `self.OuterFirearm` Firearm)
  (`|ExecutionSequence`
    (:`then_0`
      (`NiagaraFunctionLibrary.SpawnSystemAttached` "/Game/SKGSFExampleContent/Assets/Effects/MuzzleEffects/MuzzleFlash/NS_MuzzleFlash.NS_MuzzleFlash" null "S_Muzzle" _returnvalue_location _returnvalue_rotation "KeepRelativeOffset" true true "AutoRelease")
      (bind _returnvalue_2 (`GameplayStatics.SpawnEmitterAtLocation` null _returnvalue_location _returnvalue_rotation (0.5 0.5 0.5)))
      (`/Engine/EditorBlueprintResources/StandardMacros.IsValid` _returnvalue_2
        (:`Is Valid`
          (`FXSystemComponent.SetVectorParameter` _returnvalue_2 "BeamEnd" (`KismetMathLibrary.SelectVector` (`local.HitLocation`) (+ _returnvalue_location (* (`self.Range`) (`KismetMathLibrary.Conv_RotatorToVector` _returnvalue_rotation))) (`local.Hit`))))))
    (:`then_1`
      (if Hit
        (bind _returnvalue_3 (`GameplayStatics.SpawnEmitterAtLocation` (select `bool` HitPawn :!type "ParticleSystem Object Reference") HitLocation (`KismetMathLibrary.RandomRotator` false) (`KismetMathLibrary.MakeVector` _returnvalue _returnvalue _returnvalue)))
        (`GameplayStatics.SpawnSoundAttached` "/Game/SKGSFExampleContent/Assets/Effects/Audio/Raw/Shooting/UnSuppressed/A_Unsuppressed.A_Unsuppressed" _returnvalue_3 "S_Muzzle" (0.0 0.0 0.0) (struct) "KeepRelativeOffset" false 1.0 1.0 0.0 null null)))))

(fn `PreShoot`
  (bind _outercomponent (`self.OuterComponent`))
  (bind _returnvalue (`GMC_ReplicationCmp.SV_GetLastClientData` _outercomponent))
  (set `self.RemoteHitActor` null)
  (if (`GMC_ReplicationCmp.IsRemotelyControlledServerPawn` _outercomponent)
    (`self.IsValidMove` _returnvalue
      (:`True`
        (set `self.RemoteHitActor` (`GMC_ReplicationCmp.GetBoundActorReference` _outercomponent (`self.BI_RemoteHitActor`) (`.OutputState` (break `GMC_Move` _returnvalue)))))
      (:`False`
        (set `self.RemoteHitActor` null)))))

(fn `RewindTarget`
  (params (HitActor :type "Actor Object Reference"))
  (returns (ManualRewind :type Boolean))
  (bind _outercomponent (`self.OuterComponent`))
  (bind ((`Timestamp` _timestamp) (`RollbackTiming` _rollbacktiming)) (break `GMC_MetaData` (`GMC_MovementUtilityCmp.GetMoveMetaData` _outercomponent)))
  (bind _asgmc_pawn (cast `GMC_Pawn` HitActor))
  (if (!= _asgmc_pawn (`self.OuterPawn`))
    (if (`GMC_ReplicationCmp.SV_IsRewound` (`GMC_Pawn.GetReplicationComponent` _asgmc_pawn) _asgmc_pawn)
      (return false)
      (else
        (bind _asplayer_controller (cast `PlayerController` (`Pawn.GetController` (`self.OuterPawn`))))
        (bind _returnvalue (`GMC_ReplicationCmp.SV_RewindPawn` _outercomponent _asplayer_controller _timestamp _asgmc_pawn _rollbacktiming true))
        (return _returnvalue)))))

(fn `Shoot`
  (returns (Hit :type Boolean) (HitPawn :type Boolean) (HitLocation :type "Vector Structure") (HitActor :type "Actor Object Reference"))
  (locals (SV_TraceTargets :type "Array of EObjectTypeQuery Enum") (SV_BlockingObjects :type "Array of EObjectTypeQuery Enum"))
  (bind (_tracestart _traceend) (`self.GetShootingTracePoints`))
  (bind _remotehitactor (`self.RemoteHitActor`))
  (bind _remotehitactor_2 (`self.RemoteHitActor`))
  (set `self.HitActorSimulated` null)
  (set `self.SV_ShotReplicationTimer` 0.0)
  (`self.IsLocallyControlled`
    (:`true`
      _)
    (:`false`
      (if (not (`KismetSystemLibrary.IsValid` _remotehitactor_2))
        _
        (else
          (bind (_validhit _hitlocation) (`self.SV_ValidateClientShot` _remotehitactor_2 _tracestart _traceend (`local.SV_TraceTargets`) (`local.SV_BlockingObjects`)))
          (if _validhit
            (set `self.SimulateShot` true)
            (set `self.HitActorSimulated` _remotehitactor)
            (return true true _hitlocation _remotehitactor)
            (else
              (set `self.RemoteHitActor` null)
              (set `self.HitActorSimulated` null)
              (return false false (0.0 0.0 0.0) null)))))))
  (bind (_hit _hitpawn _hitlocation_2 _hitactor) (`self.ShootLocal` _tracestart _traceend))
  (set `self.SimulateShot` true)
  (if (not (`GMC_ReplicationCmp.IsRemotelyControlledServerPawn` (`self.OuterComponent`)))
    (`self.PlayShootFX` _hit _hitpawn _hitlocation_2)
    (if (`GMC_ReplicationCmp.IsAutonomousProxy` (`self.OuterComponent`))
      (`self.CL_SetHitActor` _hitactor _hitpawn)
      (else
        (set `self.HitActorSimulated` _hitactor :!label _label)))
    (else
      (goto _label)))
  (return _hit _hitpawn _hitlocation_2 _hitactor))

(fn `ShootLocal`
  (params (TraceStart :type "Vector Structure") (TraceEnd :type "Vector Structure"))
  (returns (Hit :type Boolean) (HitPawn :type Boolean) (HitLocation :type "Vector Structure") (HitActor :type "Actor Object Reference"))
  (bind _outhit (`KismetSystemLibrary.LineTraceSingle` :`Start` TraceStart :`End` TraceEnd :`TraceChannel` "TraceTypeQuery4" :`bTraceComplex` true :`DrawDebugType` "ForOneFrame" :`DrawTime` 1.0))
  (`/Engine/EditorBlueprintResources/StandardMacros.IsValid` (`.HitActor` (`GameplayStatics.BreakHitResult` _outhit))
    (:`Is Valid`
      (bind _asprimitive_component (cast `PrimitiveComponent` (`Actor.RootComponent` (`.HitActor` (`GameplayStatics.BreakHitResult` _outhit))))
        (:`then`
          (if (`|EnumEquality` (`PrimitiveComponent.GetCollisionObjectType` _asprimitive_component) "ECC_Pawn")
            (return true true (`.ImpactPoint` (`GameplayStatics.BreakHitResult` _outhit)) (`.HitActor` (`GameplayStatics.BreakHitResult` _outhit)))
            (else
              _)))
        (:`CastFailed`
          _)))
    (:`Is Not Valid`
      _))
  (return (`GameplayStatics.BreakHitResult` _outhit) false (`.ImpactPoint` (`GameplayStatics.BreakHitResult` _outhit)) (`.HitActor` (`GameplayStatics.BreakHitResult` _outhit))))

(fn `ShootSimulated`
  (bind (_tracestart _traceend) (`self.GetShootingTracePoints`))
  (bind _hitactorsimulated (`self.HitActorSimulated`))
  (bind (_hit _hitpawn _hitlocation _hitactor) (`self.ShootLocal` _tracestart _traceend))
  (if (== _hitactor _hitactorsimulated)
    (`self.PlayShootFX` _hit _hitpawn _hitlocation)
    (else
      (bind _astotw_sabot_base_pawn (cast `TOTW_SABOT_BasePawn` _hitactorsimulated)
        (:`then`
          (bind (_origin _boxextent) (`KismetSystemLibrary.GetComponentBounds` (`TOTW_MWPawn_Base.SKMesh` _astotw_sabot_base_pawn)))
          (`self.PlayShootFX` true true (`KismetMathLibrary.RandomPointInBoundingBox` _origin _boxextent)))
        (:`CastFailed`
          (`self.PlayShootFX` false))))))

(fn `ShouldApplyDamage`
  (params (HitActor :type "Actor Object Reference"))
  (returns (ShouldApplyDamage :type Boolean))
  (`/Engine/EditorBlueprintResources/ActorComponentMacros.Switch Has Authority`
    (:`Authority`
      (`/Engine/EditorBlueprintResources/StandardMacros.IsValid` HitActor
        (:`Is Valid`
          (if (`GMC_ReplicationCmp.IsRemotelyControlledServerPawn` (`self.OuterComponent`))
            (`/Engine/EditorBlueprintResources/StandardMacros.IsValid` (`self.RemoteHitActor`)
              (:`Is Valid`
                (return true))
              (:`Is Not Valid`
                _))
            (else
              (return true))))
        (:`Is Not Valid`
          _)))
    (:`Remote`
      _))
  (set `self.HitActorSimulated` null)
  (return false))

(fn `ShouldShoot`
  (params (WantsToShoot :type Boolean) (IsSemiAuto :type Boolean) (FireRate :type "Float (double-precision)") (Timestamp :type "Float (double-precision)"))
  (returns (ShouldShoot :type Boolean) (FireRatePause :type Boolean) (NumShots :type Integer))
  (locals (TimeSinceLastShot :type "Float (double-precision)") (FireInterval :type "Float (double-precision)") (RemainingTime :type "Float (double-precision)") (ShotCounter :type Integer :default 1))
  (set `local.TimeSinceLastShot` (`KismetMathLibrary.FMax` 0.0 (- Timestamp (`self.LastShotTimestamp`))))
  (set `local.FireInterval` (/ 1.0 (`KismetMathLibrary.FClamp` FireRate 0.001 1000.0)))
  (if WantsToShoot
    (if (>= (`local.TimeSinceLastShot`) (`local.FireInterval`))
      (if (not (`self.NeedsRetrigger`))
        (if (`self.IsInitialShot`)
          (set `self.IsInitialShot` false)
          (set `self.LastShotTimestamp` (`local.Timestamp`))
          (else
            (set `local.RemainingTime` (- (`local.TimeSinceLastShot`) (`local.FireInterval`)))
            (set `self.LastShotTimestamp` (`KismetMathLibrary.FMax` 0.0 (- (`local.Timestamp`) (`local.RemainingTime`))) :!label _label)
            (if (< (`local.RemainingTime`) (`local.FireInterval`))
              _
              (else
                (bind _output_get (set `local.RemainingTime` (- (stale _output_get) (`local.FireInterval`))))
                (bind _output_get_2 (set `local.ShotCounter` (+ (stale _output_get_2) 1)))
                (goto _label)))))
        (set `self.NeedsRetrigger` (`local.IsSemiAuto`))
        (return true false (`local.ShotCounter`))
        (else
          _))
      (else
        (return false true 0)))
    (else
      (set `self.IsInitialShot` true)
      (set `self.NeedsRetrigger` false)))
  (return false false 0))

(fn `SV_ValidateClientShot`
  (params (HitActor :type "Actor Object Reference") (TraceStart :type "Vector Structure") (TraceEnd :type "Vector Structure") (TargetObjectTypes :type "Array of EObjectTypeQuery Enum (by ref)") (BlockingObjectTypes :type "Array of EObjectTypeQuery Enum"))
  (returns (ValidHit :type Boolean) (HitLocation :type "Vector Structure"))
  (locals (ActorHitLocation :type "Vector Structure"))
  (bind _tracestart (`local.TraceStart`))
  (bind _manualrewind (`self.RewindTarget` HitActor))
  (bind _outhits (`KismetSystemLibrary.SphereTraceMultiForObjects` :`Start` TraceStart :`End` TraceEnd :`Radius` (`self.SV_ValidationRadius`) :`ObjectTypes` TargetObjectTypes :`TraceColor` (struct :`B` 1.0 :`A` 1.0) :`TraceHitColor` (struct :`R` 1.0 :`G` 1.0 :`A` 1.0) :`DrawTime` 1.0))
  (if _manualrewind
    (`self.UnwindTarget` (`self.RemoteHitActor`)))
  (for _array_element _outhits
    (if (`self.ValidateHitActor` _array_element (`local.HitActor`))
      (set `local.ActorHitLocation` (`.ImpactPoint` (`GameplayStatics.BreakHitResult` _array_element)))
      (bind (_outhit _returnvalue) (`KismetSystemLibrary.LineTraceSingleForObjects` :`Start` (`local.TraceStart`) :`End` (`local.TraceEnd`) :`ObjectTypes` (`local.BlockingObjectTypes`) :`TraceColor` (struct :`B` 1.0 :`A` 1.0) :`TraceHitColor` (struct :`R` 1.0 :`G` 1.0 :`A` 1.0) :`DrawTime` 1.0))
      (if (not _returnvalue)
        _
        (elif (>= (`KismetMathLibrary.Vector_Distance` (`.ImpactPoint` (`GameplayStatics.BreakHitResult` _outhit)) _tracestart) (`KismetMathLibrary.Vector_Distance` _tracestart (`local.ActorHitLocation`)))
          _
          (else
            (return false (0.0 0.0 0.0)))))
      (return true (`local.ActorHitLocation`))))
  (return false (0.0 0.0 0.0)))

(fn `UnwindTarget`
  (params (HitActor :type "Actor Object Reference"))
  (bind _asgmc_pawn (cast `GMC_Pawn` HitActor))
  (if (`GMC_ReplicationCmp.SV_IsRewound` (`GMC_Pawn.GetReplicationComponent` _asgmc_pawn) _asgmc_pawn)
    (cast `PlayerController` (`Pawn.GetController` (`self.OuterPawn`)))
    (`GMC_ReplicationCmp.SV_RestorePawnAfterRewind` (`self.OuterComponent`) _asgmc_pawn true)))

(fn `UpdateAttributes`
  (params (SemiAuto :type Boolean) (FireRate :type "Float (double-precision)") (Damage :type "Float (double-precision)") (Range :type "Float (double-precision)"))
  (set `self.SemiAuto` SemiAuto)
  (set `self.FireRate` FireRate)
  (set `self.Damage` Damage)
  (set `self.Range` Range))

(fn `ValidateHitActor`
  (params (Hit :type "HitResult Structure (by ref)") (RemoteHitActor :type "Actor Object Reference"))
  (returns (ActorValidated :type Boolean))
  (bind (_bblockinghit _binitialoverlap _time _distance _location _impactpoint _normal _impactnormal _physmat _hitactor) (`GameplayStatics.BreakHitResult` Hit))
  (return (and _bblockinghit (== _hitactor RemoteHitActor))))