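; Template player character for a shooter, combining an SKG shooter pawn, an ability system with health, death and respawn, and first/third-person cameras.
; Input drives firing, leaning, procedural weapon poses, queued jump and roll abilities, and sweep-based pickup and drop.
; Zero health triggers ragdoll and a respawn widget, with jump respawning.
; Tick updates status aura effects and state-based camera blending; mesh setup routes through the server.
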(event `SpawnDefaultFirearm`
  (`/Engine/EditorBlueprintResources/ActorMacros.Switch Has Authority`
    (:`Authority`
      (bind _returnvalue (`|SpawnActorFromClass` "/Game/SKGSFExampleContent/Blueprints/Firearms/Premade/M4/BP_M4.BP_M4_C" (`KismetMathLibrary.MakeTransform` (0.0 0.0 0.0)) "AlwaysSpawn" "MultiplyWithRoot" self "/Game/SKGSFExampleContent/Data/FirearmConstruction/Firearms/M4/DA_M4.DA_M4" null))
      (`self.K2_AttachToComponent` _returnvalue (`self.SKMesh`) "ik_hand_gun" "SnapToTarget" "SnapToTarget" "SnapToTarget" true)
      (`SKGShooterPawnComponent.SetHeldActor` (`self.SKGShooterPawn`) _returnvalue))))

(event `self.ReceiveBeginPlay`
  (`parent.ReceiveBeginPlay`)
  (add `GMC_AbilitySystemComponent.OnAttributeChanged` (`self.AbilitySystemComponent`) (delegate `OnAttributeChanged`))
  (`self.Setup`)
  (`self.Set_TPFP_Cam` (`self.bIsFirstPerson`))
  (`self.Mesh_Setup_Start` null))

(event `EnhancedInput|/Game/GMASExtended/Input/IA_Jump`
  (params (ActionValue :type Boolean) (ElapsedSeconds :type "Float (double-precision)") (TriggeredSeconds :type "Float (double-precision)") (InputAction :type "InputAction Object Reference" :default "/Game/GMASExtended/Input/IA_Jump.IA_Jump"))
  ;[0.01096 0.01161 0.0137] InputActions
  (:`Started`
    (`self.HandleJump` InputAction)))

(event `OnAttributeChanged`
  (params (AttributeTag :type "GameplayTag Structure") (OldValue :type "Float (single-precision)") (NewValue :type "Float (single-precision)"))
  (if (and (== AttributeTag (struct :`TagName` "Attribute.Health")) (> OldValue 0.0) (<= NewValue 0.0))
    (`self.HandleDeath`)
    (add `SKGShooterPawnComponent.OnPoseComplete` (`self.SKGShooterPawn`) (`|CreateDelegate` :!event `OnPoseComplete`))))

(event `EnhancedInput|/Game/GMASExtended/Input/IA_Roll`
  (params (ActionValue :type Boolean) (ElapsedSeconds :type "Float (double-precision)") (TriggeredSeconds :type "Float (double-precision)") (InputAction :type "InputAction Object Reference" :default "/Game/GMASExtended/Input/IA_Roll.IA_Roll"))
  ;[0.01096 0.01161 0.0137] InputActions
  (:`Triggered`
    (`GMC_AbilitySystemComponent.QueueAbility` (`self.AbilitySystemComponent`) (struct :`TagName` "Ability.Roll") InputAction)))

(event `self.ReceiveTick`
  (params (DeltaSeconds :type "Float (single-precision)"))
  (`parent.ReceiveTick` DeltaSeconds)
  (`self.ShowStatusEffects`)
  (if (`self.AutomaticCameraEnable`)
    (`self.SetCameraByState`)
    (`self.UpdateCamera` true)))

(event `self.OnRespawn`
  (bind _abilitysystemcomponent (`self.AbilitySystemComponent`))
  (bind _respawnwidget (`self.RespawnWidget`))
  (bind _abilitysystemcomponent_2 (`self.AbilitySystemComponent`))
  (`GMCE_OrganicMovementCmp.DisableRagdoll` (`self.Template Movement Component`))
  ;[0.1188 1 0.1619] Reset health and stamina attributes to max values.
  (`GMC_AbilitySystemComponent.SetAttributeValueByTag` _abilitysystemcomponent (struct :`TagName` "Attribute.Health") (`GMC_AbilitySystemComponent.GetAttributeValueByTag` _abilitysystemcomponent_2 (struct :`TagName` "Attribute.HealthMax")) true)
  (`GMC_AbilitySystemComponent.SetAttributeValueByTag` _abilitysystemcomponent (struct :`TagName` "Attribute.Stamina") (`GMC_AbilitySystemComponent.GetAttributeValueByTag` _abilitysystemcomponent_2 (struct :`TagName` "Attribute.StaminaMax")) true)
  ;[1 0.05949 0.7813] Remove the respawn overlay widget (if we have one).
  (`/Engine/EditorBlueprintResources/StandardMacros.IsValid` _respawnwidget
    (:`Is Valid`
      (`Widget.RemoveFromParent` _respawnwidget)
      (set `self.RespawnWidget` null))))

(event `EquipFirearm`
  (params (Firearm :type "Actor Object Reference"))
  (`/Engine/EditorBlueprintResources/ActorMacros.Switch Has Authority`
    (:`Authority`
      (`self.K2_AttachToComponent` Firearm (`self.SKMesh`) (`self.FirearmAttachSocket`) "SnapToTarget" "SnapToTarget" "SnapToTarget" true)
      (`SKGShooterPawnComponent.SetHeldActor` (`self.SKGShooterPawn`) Firearm)
      (message `/Game/SKGSFExampleContent/Blueprints/Interfaces/BPI_Interaction.SetOwningPawn` Firearm self))))

(event `EnhancedInput|/Game/GMASExtended/Input/IA_PointAiming`
  (params (ActionValue :type Boolean) (ElapsedSeconds :type "Float (double-precision)") (TriggeredSeconds :type "Float (double-precision)") (InputAction :type "InputAction Object Reference" :default "/Game/GMASExtended/Input/IA_PointAiming.IA_PointAiming"))
  (bind _returnvalue (`SKGShooterPawnComponent.GetCurrentFirearmComponent` (`self.SKGShooterPawn`)))
  (:`Started`
    (if (`SKGFirearmComponent.IsPointAiming` _returnvalue)
      (`SKGFirearmComponent.StopPointAiming` _returnvalue (`SKGShooterPawnComponent.bIsAiming` (`self.SKGShooterPawn`)))
      (else
        (`SKGFirearmComponent.StartPointAiming` _returnvalue true)))))

(event `EnhancedInput|/Game/GMASExtended/Input/IA_Fire`
  (params (ActionValue :type Boolean) (ElapsedSeconds :type "Float (double-precision)") (TriggeredSeconds :type "Float (double-precision)") (InputAction :type "InputAction Object Reference" :default "/Game/GMASExtended/Input/IA_Fire.IA_Fire"))
  (bind _heldactor (`SKGShooterPawnComponent.HeldActor` (`self.SKGShooterPawn`)))
  (:`Started`
    (`/Engine/EditorBlueprintResources/StandardMacros.IsValid` _heldactor
      (:`Is Valid`
        (message `/Game/SKGSFExampleContent/Blueprints/Interfaces/BPI_Firearm.PressTrigger` _heldactor))))
  (:`Canceled`
    (`/Engine/EditorBlueprintResources/StandardMacros.IsValid` _heldactor :!label _label
      (:`Is Valid`
        (message `/Game/SKGSFExampleContent/Blueprints/Interfaces/BPI_Firearm.ReleaseTrigger` _heldactor))))
  (:`Completed`
    (goto _label)))

(event `EnhancedInput|/Game/GMASExtended/Input/IA_LeanLeft`
  (params (ActionValue :type Boolean) (ElapsedSeconds :type "Float (double-precision)") (TriggeredSeconds :type "Float (double-precision)") (InputAction :type "InputAction Object Reference" :default "/Game/GMASExtended/Input/IA_LeanLeft.IA_LeanLeft"))
  (bind _skgshooterpawn (`self.SKGShooterPawn`))
  (:`Started`
    (`SKGShooterPawnComponent.LeanLeft` _skgshooterpawn (`self.LeanAmount`)))
  (:`Canceled`
    (`SKGShooterPawnComponent.StopLeaningLeft` _skgshooterpawn :!label _label))
  (:`Completed`
    (goto _label)))

(event `EnhancedInput|/Game/GMASExtended/Input/IA_LeanRight`
  (params (ActionValue :type Boolean) (ElapsedSeconds :type "Float (double-precision)") (TriggeredSeconds :type "Float (double-precision)") (InputAction :type "InputAction Object Reference" :default "/Game/GMASExtended/Input/IA_LeanRight.IA_LeanRight"))
  (bind _skgshooterpawn (`self.SKGShooterPawn`))
  (:`Started`
    (`SKGShooterPawnComponent.LeanRight` _skgshooterpawn (`self.LeanAmount`)))
  (:`Canceled`
    (`SKGShooterPawnComponent.StopLeaningRight` _skgshooterpawn :!label _label_2))
  (:`Completed`
    (goto _label_2)))

(event `EnhancedInput|/Game/GMASExtended/Input/IA_Drop`
  (params (ActionValue :type Boolean) (ElapsedSeconds :type "Float (double-precision)") (TriggeredSeconds :type "Float (double-precision)") (InputAction :type "InputAction Object Reference" :default "/Game/GMASExtended/Input/IA_Drop.IA_Drop"))
  (bind _heldactor (`SKGShooterPawnComponent.HeldActor` (`self.SKGShooterPawn`)))
  (:`Started`
    (`/Engine/EditorBlueprintResources/StandardMacros.IsValid` _heldactor
      (:`Is Valid`
        (`self.DropActor` _heldactor)))))

(event `EnhancedInput|/Game/GMASExtended/Input/IA_Interact`
  (params (ActionValue :type Boolean) (ElapsedSeconds :type "Float (double-precision)") (TriggeredSeconds :type "Float (double-precision)") (InputAction :type "InputAction Object Reference" :default "/Game/GMASExtended/Input/IA_Interact.IA_Interact"))
  (bind _fp_cam (`self.FP_Cam`))
  ;[1 1 1] Perform a sweep, if our sweep hits an actor, walk up to the most outer parent (such as if you hit the optic of the m4, walk up the outer chain until you hit the upper most parent (the m4 if it has no owner)) and if that parent implements the BPI_Interact interface, it is a valid interaction
  (:`Started`
    (bind _hitactor (`self.PerformInteractionSweep` (`SceneComponent.K2_GetComponentLocation` _fp_cam) (`SceneComponent.GetForwardVector` _fp_cam)))
    (`/Engine/EditorBlueprintResources/StandardMacros.IsValid` _hitactor
      (:`Is Valid`
        (`/Engine/EditorBlueprintResources/ActorMacros.Switch Has Authority`
          (:`Authority`
            (`self.HandleInteraction` _hitactor))
          (:`Remote`
            (`self.Server_HandleInteraction` _hitactor)))))))

(event `Server_HandleInteraction`
  (params (Actor :type "Actor Object Reference"))
  (`self.HandleInteraction` Actor))

(event `HandleInteraction`
  (params (Actor :type "Actor Object Reference"))
  (bind _bpickup (message `/Game/SKGSFExampleContent/Blueprints/Interfaces/BPI_Interaction.IsPickup` Actor))
  (if _bpickup
    (`self.PickupActor` Actor))
  (message `/Game/SKGSFExampleContent/Blueprints/Interfaces/BPI_Interaction.Interact` Actor self))

(event `PickupActor`
  (params (Actor :type "Actor Object Reference"))
  (bind _heldactor (`SKGShooterPawnComponent.HeldActor` (`self.SKGShooterPawn`)))
  (`/Engine/EditorBlueprintResources/StandardMacros.IsValid` _heldactor
    (:`Is Valid`
      (`self.DropActor` _heldactor))
    (:`Is Not Valid`
      _))
  (`self.EquipFirearm` Actor))

(event `DropActor`
  (params (Actor :type "Actor Object Reference"))
  (`SKGShooterPawnComponent.ClearHeldActor` (`self.SKGShooterPawn`))
  (message `/Game/SKGSFExampleContent/Blueprints/Interfaces/BPI_Interaction.Drop` Actor))

(event `Server_ReplicateNodsState`
  (params (bFlippedDown :type Boolean))
  (set `self.bNodsFlippedDown` bFlippedDown))

(event `Key|G`
  (params (Key :type "Key Structure"))
  (:`Pressed`
    (bind _returnvalue (`|CreateWidget` "/Game/SKGSFExampleContent/UI/PoseCustomization/WBP_PoseCustomization.WBP_PoseCustomization_C"))
    (`UserWidget.AddToViewport` _returnvalue 0)))

(event `OnPoseComplete`
  (params (CurrentPoseData :type "SKGProceduralPoseReplicationData Structure (by ref)"))
  (set `self.bIsPerformingPose` false))

(event `TryGoToPose`
  (params (Tag :type "GameplayTag Structure"))
  (bind _skgshooterpawn (`self.SKGShooterPawn`))
  (bind (_currentproceduralposedata_tag _currentproceduralposedata_bexitpose) (break `SKGProceduralPoseReplicationData` (`SKGShooterPawnComponent.CurrentProceduralPoseData` _skgshooterpawn)))
  ;[1 1 1] If in current pose, exit pose. Once pose is exited, you can go to a new pose
  (if _currentproceduralposedata_bexitpose
    (`SKGShooterPawnComponent.PerformProceduralPose` _skgshooterpawn Tag false :!label _label)
    (elif (`BlueprintGameplayTagLibrary.IsGameplayTagValid` _currentproceduralposedata_tag)
      (`SKGShooterPawnComponent.PerformProceduralPose` _skgshooterpawn _currentproceduralposedata_tag true)
      (else
        (goto _label)))))

(event `EnhancedInput|/Game/GMASExtended/Input/IA_HighPort`
  (params (ActionValue :type Boolean) (ElapsedSeconds :type "Float (double-precision)") (TriggeredSeconds :type "Float (double-precision)") (InputAction :type "InputAction Object Reference" :default "/Game/GMASExtended/Input/IA_HighPort.IA_HighPort"))
  (:`Started`
    (if (`self.bIsPerformingPose`) :!label _label_2
      _
      (elif (not (`SKGShooterPawnComponent.bIsAiming` (`self.SKGShooterPawn`)))
        (`self.TryGoToPose` (struct :`TagName` "Poses.HighPort"))
        (set `self.bIsPerformingPose` true)))))

(event `Key|MouseScrollUp`
  (params (Key :type "Key Structure"))
  ; Temp fix
  (:`Pressed`
    (goto _label_2)))

(event `EnhancedInput|/Game/GMASExtended/Input/IA_LowPort`
  (params (ActionValue :type Boolean) (ElapsedSeconds :type "Float (double-precision)") (TriggeredSeconds :type "Float (double-precision)") (InputAction :type "InputAction Object Reference" :default "/Game/GMASExtended/Input/IA_LowPort.IA_LowPort"))
  (:`Triggered`
    (if (`self.bIsPerformingPose`) :!label _label_3
      _
      (elif (not (`SKGShooterPawnComponent.bIsAiming` (`self.SKGShooterPawn`)))
        (`self.TryGoToPose` (struct :`TagName` "Poses.LowPort"))
        (set `self.bIsPerformingPose` true)))))

(event `Key|MouseScrollDown`
  (params (Key :type "Key Structure"))
  ; Temp fix
  (:`Pressed`
    (goto _label_3)))

(event `EnhancedInput|/Game/GMASExtended/Input/IA_ShortStock`
  (params (ActionValue :type Boolean) (ElapsedSeconds :type "Float (double-precision)") (TriggeredSeconds :type "Float (double-precision)") (InputAction :type "InputAction Object Reference" :default "/Game/GMASExtended/Input/IA_ShortStock.IA_ShortStock"))
  (:`Started`
    (if (`self.bIsPerformingPose`)
      _
      (elif (not (`SKGShooterPawnComponent.bIsAiming` (`self.SKGShooterPawn`)))
        (`self.TryGoToPose` (struct :`TagName` "Poses.ShortStock"))
        (set `self.bIsPerformingPose` true)))))

(event `EnhancedInput|/Game/SKGSFExampleContent/Input/Actions/Firearm/Poses/IA_BlindFire`
  (params (ActionValue :type Boolean) (ElapsedSeconds :type "Float (double-precision)") (TriggeredSeconds :type "Float (double-precision)") (InputAction :type "InputAction Object Reference" :default "/Game/SKGSFExampleContent/Input/Actions/Firearm/Poses/IA_BlindFire.IA_BlindFire"))
  ; Still needs replacing
  (:`Started`
    (if (`self.bIsPerformingPose`)
      _
      (elif (not (`SKGShooterPawnComponent.bIsAiming` (`self.SKGShooterPawn`)))
        (`self.TryGoToPose` (struct :`TagName` "Poses.BlindFire"))
        (set `self.bIsPerformingPose` true)))))

(event `SRVR_MeshSetup`
  (params (NewMesh :type "SkeletalMesh Object Reference") (AnimInstance :type "AnimInstance Class Reference"))
  ;[0.2306 1 0.1068] Mesh Change Replication
  (`self.CL_MeshSetup` NewMesh AnimInstance))

(event `CL_MeshSetup`
  (params (NewMesh :type "SkeletalMesh Object Reference") (AnimInstance :type "AnimInstance Class Reference"))
  (bind _skmesh (`self.SKMesh`))
  ;[0.2306 1 0.1068] Mesh Change Replication
  (`SkeletalMeshComponent.SetSkeletalMeshAsset` _skmesh NewMesh)
  (`KismetSystemLibrary.Delay` 0.2)
  (`SkeletalMeshComponent.SetAnimInstanceClass` _skmesh AnimInstance))

(event `Mesh_Setup_Start`
  (params (NewMesh :type "SkeletalMesh Object Reference") (AnimInstance :type "AnimInstance Class Reference"))
  ;[0.2306 1 0.1068] Mesh Change Replication
  ;;[1 0 0] DISCONNECT TO NOT LOAD FROM DA
  (`/Engine/EditorBlueprintResources/ActorMacros.Switch Has Authority`
    (:`Authority`
      (`self.CL_MeshSetup` NewMesh AnimInstance))
    (:`Remote`
      (`self.SRVR_MeshSetup` NewMesh AnimInstance))))

(fn `HandleDeath`
  (`GMC_AbilitySystemComponent.AddActiveTag` (`self.AbilitySystemComponent`) (struct :`TagName` "State.Dead"))
  (`GMCE_OrganicMovementCmp.EnableRagdoll` (`self.Template Movement Component`))
  (if (and (`self.IsLocallyControlled`) (not (`KismetSystemLibrary.IsValid` (`self.RespawnWidget`))))
    (bind _returnvalue (`|CreateWidget` "/Game/GMASExtended/UI/WBP_Respawn.WBP_Respawn_C" (`GameplayStatics.GetPlayerControllerFromID` 0)))
    (bind _output_get (set `self.RespawnWidget` _returnvalue))
    (`UserWidget.AddToViewport` _output_get 1)))

(fn `HandleJump`
  (params (InputAction :type "InputAction Object Reference"))
  (if (`GMC_AbilitySystemComponent.HasActiveTag` (`self.AbilitySystemComponent`) (struct :`TagName` "State.Dead"))
    (`self.Respawn`)
    (else
      (`GMC_AbilitySystemComponent.QueueAbility` (`self.AbilitySystemComponent`) (struct :`TagName` "Ability.Jump") InputAction))))

(fn `PerformInteractionSweep`
  (params (TraceStart :type "Vector Structure") (TraceDirection :type "Vector Structure"))
  (returns (HitActor :type "Actor Object Reference"))
  (locals (ParentActor :type "Actor Object Reference") (TempParent :type "Actor Object Reference"))
  (bind _parentactor (`local.ParentActor`))
  (bind _outhit (`KismetSystemLibrary.SphereTraceSingle` TraceStart (+ TraceStart (* TraceDirection (`self.InteractionSweepDistance`))) (`self.InteractionSweepRadius`) "TraceTypeQuery1" false (`self.GetAttachedActors` false true) "ForDuration"))
  (bind (_bblockinghit _binitialoverlap _time _distance _location _impactpoint _normal _impactnormal _physmat _hitactor) (`GameplayStatics.BreakHitResult` _outhit))
  (if _bblockinghit
    (bind _output_get (set `local.ParentActor` _hitactor))
    (set `local.TempParent` _output_get)
    (while (`KismetSystemLibrary.IsValid` (`local.TempParent`))
      (bind _output_get_2 (set `local.TempParent` (`self.GetOwner` (`local.TempParent`))))
      (`/Engine/EditorBlueprintResources/StandardMacros.IsValid` _output_get_2
        (:`Is Valid`
          (set `local.ParentActor` _output_get_2))))
    (if (`KismetSystemLibrary.DoesImplementInterface` _parentactor "/Game/SKGSFExampleContent/Blueprints/Interfaces/BPI_Interaction.BPI_Interaction_C")
      (return _parentactor)
      (else
        (return null)))
    (else
      (return null))))

(fn `Set_TPFP_Cam`
  (params (`FP ?` :type Boolean))
  (if `FP ?`
    (`ActorComponent.SetActive` (`self.TPCam`) false false)
    (`ActorComponent.SetActive` (`self.FP_Cam`) true false)
    (else
      (`ActorComponent.SetActive` (`self.FP_Cam`) false false)
      (`ActorComponent.SetActive` (`self.TPCam`) true false))))

(fn `SetCameraByState`
  (bind _abilitysystemcomponent (`self.AbilitySystemComponent`))
  (if (`GMC_AbilitySystemComponent.HasActiveTag` _abilitysystemcomponent (struct :`TagName` "State.IsAiming"))
    (set `self.ActiveCameraSettings` (`self.Camera_Aim`))
    (elif (`GMC_AbilitySystemComponent.HasActiveTag` _abilitysystemcomponent (struct :`TagName` "State.IsStrafing"))
      (set `self.ActiveCameraSettings` (`self.Camera_Strafe`))
      (else
        (set `self.ActiveCameraSettings` (`self.Camera_Default`))))))

(fn `Setup`
  (bind _asgmc_player_controller (cast `GMC_PlayerController` (`GameplayStatics.GetPlayerControllerFromID` 0)))
  (bind _returnvalue (`|CreateWidget` "/Game/GMASExtended/UI/WBP_HUD.WBP_HUD_C" _asgmc_player_controller))
  (bind _output_get (set `self.StatusWidget` _returnvalue))
  (`UserWidget.AddToViewport` _returnvalue 0)
  (`UserWidget.AddToViewport` _output_get 0))

(fn `ShowStatusEffects`
  (bind _status_aura (`self.Status_Aura`))
  (bind _status_aura_2 (`self.Status_Aura`))
  (bind _returnvalue (`GMC_AbilitySystemComponent.HasActiveTag` (`self.AbilitySystemComponent`) (struct :`TagName` "State.Healing")))
  (bind _returnvalue_2 (`KismetMathLibrary.SelectColor` (struct :`G` 0.630208 :`A` 1.0) (struct :`R` 0.855903 :`A` 1.0) _returnvalue))
  (if (`GMC_AbilitySystemComponent.HasAnyTag` (`self.AbilitySystemComponent`) (struct :`GameplayTags` (struct :`(TagName` "State.Burning") :`(TagName` "State.Healing"))))
    (if (!= (`self.HasHealAura`) _returnvalue)
      (`NiagaraComponent.ResetSystem` (`self.Status_Aura`)))
    (set `self.HasHealAura` _returnvalue)
    ;[0.2793 0.3872 0.1097] Set up particle system and overlay material
    (`NiagaraComponent.SetVariableLinearColor` _status_aura "Color" _returnvalue_2)
    (`NiagaraComponent.SetVariableFloat` _status_aura "SpawnRate" (`KismetMathLibrary.SelectFloat` 0.0 120.0 _returnvalue))
    (`NiagaraComponent.SetVariableBool` _status_aura "UseOrbiters" _returnvalue)
    (`NiagaraFunctionLibrary.OverrideSystemUserVariableSkeletalMeshComponent` _status_aura "" (`self.SKMesh`))
    (`NiagaraComponent.SetVariableBool` _status_aura "UseFlames" (not (`self.HasHealAura`)))
    (`ActorComponent.Activate` _status_aura false)
    (bind _returnvalue_3 (`KismetMaterialLibrary.CreateDynamicMaterialInstance` "/Game/GMASExtended/Particles/M_Aura_Overlay.M_Aura_Overlay" "None" "Transient"))
    (`MaterialInstanceDynamic.SetVectorParameterValue` _returnvalue_3 "Color" _returnvalue_2)
    (`MeshComponent.SetOverlayMaterial` (`self.SKMesh`) _returnvalue_3)
    (else
      (`NiagaraComponent.SetVariableBool` _status_aura_2 "UseFlames" false)
      (`NiagaraComponent.SetVariableBool` _status_aura_2 "UseOrbiters" false)
      (`ActorComponent.Deactivate` _status_aura_2)
      (`MeshComponent.SetOverlayMaterial` (`self.SKMesh`) null))))

(fn `UpdateCamera`
  (params (Interpolate :type Boolean))
  (locals (TemporaryCameraSettings :type "/Game/GMASExtended/Data/S_CameraParameters Structure"))
  (bind (_activecamerasettings_springarmlength _activecamerasettings_fieldofview _activecamerasettings_transitionspeed _activecamerasettings_socketoffset _activecamerasettings_translationlagspeed) (break `/Game/GMASExtended/Data/S_CameraParameters` (`self.ActiveCameraSettings`)))
  (bind (_temporarycamerasettings_springarmlength _temporarycamerasettings_fieldofview _temporarycamerasettings_transitionspeed) (break `/Game/GMASExtended/Data/S_CameraParameters` (`local.TemporaryCameraSettings`)))
  (bind (_temporarycamerasettings_springarmlength_2 _temporarycamerasettings_fieldofview_2 _temporarycamerasettings_transitionspeed_2 _temporarycamerasettings_socketoffset) (break `/Game/GMASExtended/Data/S_CameraParameters` (`local.TemporaryCameraSettings`)))
  (bind (_temporarycamerasettings_springarmlength_3 _temporarycamerasettings_fieldofview_3 _temporarycamerasettings_transitionspeed_3 _temporarycamerasettings_socketoffset_2 _temporarycamerasettings_translationlagspeed) (break `/Game/GMASExtended/Data/S_CameraParameters` (`local.TemporaryCameraSettings`)))
  (bind _interpolate (`local.Interpolate`))
  (bind (_temporarycamerasettings_springarmlength_4 _temporarycamerasettings_fieldofview_4 _temporarycamerasettings_transitionspeed_4) (break `/Game/GMASExtended/Data/S_CameraParameters` (`local.TemporaryCameraSettings`)))
  (set `local.TemporaryCameraSettings` (make `/Game/GMASExtended/Data/S_CameraParameters` _activecamerasettings_springarmlength _activecamerasettings_fieldofview (`KismetMathLibrary.SelectFloat` _activecamerasettings_transitionspeed -1.0 _interpolate) _activecamerasettings_socketoffset (`KismetMathLibrary.SelectFloat` _activecamerasettings_translationlagspeed -1.0 _interpolate)))
  (bind _output_get (set `CameraComponent.FieldOfView` (`KismetMathLibrary.FInterpTo` (stale _output_get) _temporarycamerasettings_fieldofview_4 (`GameplayStatics.GetWorldDeltaSeconds`) _temporarycamerasettings_transitionspeed_4) (`self.TPCam`)))
  (bind _output_get_2 (set `SpringArmComponent.TargetArmLength` (`KismetMathLibrary.FInterpTo` (stale _output_get_2) _temporarycamerasettings_springarmlength (`GameplayStatics.GetWorldDeltaSeconds`) _temporarycamerasettings_transitionspeed) (`self.TPArm`)))
  (bind _output_get_3 (set `SpringArmComponent.SocketOffset` (`KismetMathLibrary.VInterpTo` (stale _output_get_3) _temporarycamerasettings_socketoffset (`GameplayStatics.GetWorldDeltaSeconds`) _temporarycamerasettings_transitionspeed_2) (`self.TPArm`)))
  (bind _output_get_4 (set `SpringArmComponent.CameraLagSpeed` (`KismetMathLibrary.FInterpTo` (stale _output_get_4) _temporarycamerasettings_translationlagspeed (`GameplayStatics.GetWorldDeltaSeconds`) _temporarycamerasettings_transitionspeed_3) (`self.TPArm`))))

(fn `UserConstructionScript`
  (`parent.UserConstructionScript`))