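; Player controller for a GMC-based character that sets camera limits and handles input for a firearm customizer UI.
; On BeginPlay it clamps the camera manager's view pitch to a symmetric range.
; The customizer input toggles the panel on the main widget if that is valid.
; The local-only main UI setup is disconnected from BeginPlay, and it assigns None instead of the created motion-match widget.
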(event `self.ReceiveBeginPlay`
  (`self.SetCameraLimits`))

(event `SetCameraLimits`
  (bind _playercameramanager (`self.PlayerCameraManager`))
  (set `PlayerCameraManager.ViewPitchMin` -75.0 _playercameramanager)
  (set `PlayerCameraManager.ViewPitchMax` 75.0 _playercameramanager))

(event `AddMainUI`
  (if (`self.IsLocalController`)
    (`|CreateWidget` "/GMCE_Motion/UI/WBP_MotionMatch.WBP_MotionMatch_C")
    (bind _output_get (set `self.WBP_Main` null))
    (`UserWidget.AddToViewport` _output_get 0)))

(event `EnhancedInput|/Game/GMASExtended/Input/IA_Customiser`
  (params (ActionValue :type Boolean) (ElapsedSeconds :type "Float (double-precision)") (TriggeredSeconds :type "Float (double-precision)") (InputAction :type "InputAction Object Reference" :default "/Game/GMASExtended/Input/IA_Customiser.IA_Customiser"))
  (bind _wbp_main (`self.WBP_Main`))
  (:`Triggered`
    (`/Engine/EditorBlueprintResources/StandardMacros.IsValid` _wbp_main
      (:`Is Valid`
        (`/Game/SKGSFExampleContent/UI/WBP_Main.ToggleFirearmCustomizer` _wbp_main)))))

(fn `UserConstructionScript`)